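; BP_P38 is a player-controlled P-38 plane that constantly flies forward, steers with pitch and roll, and fires projectiles.
; Tick feeds movement input along the forward vector, while the Pitch and Roll axes apply local rotation scaled by delta time and RotateSpeed.
; BeginPlay registers both propeller meshes with BPRotateSceneComponent, presumably to spin them.
; Pressing Fire spawns a BP_Rocke at the plane's own transform.
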(event EventBeginPlay
  (Utilities|Array|Add (Variables|/Game/BluePrint/BP_RotateSceneComponent.BP_RotateSceneComponent_C|GetSceneComponent (Variables|Default|GetBP_RotateSceneComponent)) (Variables|Default|GetSM_P38_Right_Propeller))
  (Utilities|Array|Add (Variables|/Game/BluePrint/BP_RotateSceneComponent.BP_RotateSceneComponent_C|GetSceneComponent (Variables|Default|GetBP_RotateSceneComponent)) (Variables|Default|GetSM_P38_Left_Propeller)))

(event EventTick
  (params (DeltaSeconds :type Float%20%28single-precision%29))
  (Pawn|Input|AddMovementInput (Transformation|GetActorForwardVector) 1.0 false))

(event Input|ActionEvents|InputActionFire
  (params (Key :type Key%20Structure :default "None"))
  (:Pressed
    (Game|SpawnActorfromClass "/Game/BluePrint/Roketet/BP_Rocke.BP_Rocke_C" (Transformation|GetActorTransform) "Undefined" "MultiplyWithRoot" 0 0)))

(event Input|AxisEvents|InputAxisPitch
  (params (AxisValue :type Float%20%28single-precision%29))
  (Transformation|AddActorLocalRotation (Math|Rotator|MakeRotator 0.0 (* AxisValue (Utilities|Time|GetWorldDeltaSeconds) (Variables|Default|GetRotateSpeed)) 0.0) false false))

(event Input|AxisEvents|InputAxisRoll
  (params (AxisValue :type Float%20%28single-precision%29))
  (Transformation|AddActorLocalRotation (Math|Rotator|MakeRotator (* AxisValue (Utilities|Time|GetWorldDeltaSeconds) (Variables|Default|GetRotateSpeed)) 0.0 0.0) false false))

(fn ConstructionScript)